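; Enemy NPC that melee-attacks the player and awards score when killed.
; Hits reduce Health and spawn sparks until death, which stops AI and movement, then destroys the actor after a delay.
; Kills award points through the player's multiplier, with temporary bonuses for grapple, mid-air and no-scope kills, flagged for Tick to flash HUD messages.
; Attacks play a throttled sound and damage the player if still in range after a delay.
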(event `self.ReceiveTick`
  (params (DeltaSeconds :type "Float (single-precision)"))
  (bind _grapplemessage (`/Game/UI/PointSystem/PointUI.Grapplemessage` (`/Game/FirstPerson/Blueprints/BP_FirstPersonCharacter.PointHUD` (`self.As BP First Person Character`))))
  (bind _midairmessage (`/Game/UI/PointSystem/PointUI.Midairmessage` (`/Game/FirstPerson/Blueprints/BP_FirstPersonCharacter.PointHUD` (`self.As BP First Person Character`))))
  (bind _noscopemessage (`/Game/UI/PointSystem/PointUI.Noscopemessage` (`/Game/FirstPerson/Blueprints/BP_FirstPersonCharacter.PointHUD` (`self.As BP First Person Character`))))
  (set `self.Delta Seconds` DeltaSeconds)
  (`|ExecutionSequence`
    (:`then_0`
      (if (`self.MidAirMessage`)
        (`Widget.SetRenderOpacity` _midairmessage 1.0)
        (`KismetSystemLibrary.Delay` 1.0)
        (`Widget.SetRenderOpacity` _midairmessage 0.0)
        (set `self.MidAirMessage` false)
        (elif (`self.GrappleMessage`)
          (`Widget.SetRenderOpacity` _grapplemessage 1.0)
          (`KismetSystemLibrary.Delay` 1.0)
          (`Widget.SetRenderOpacity` _grapplemessage 0.0)
          (set `self.GrappleMessage` false))))
    (:`then_1`
      (if (`self.NoScopeMessage`)
        (`Widget.SetRenderOpacity` _noscopemessage 1.0)
        (`KismetSystemLibrary.Delay` 1.0)
        (`Widget.SetRenderOpacity` _noscopemessage 0.0)
        (set `self.NoScopeMessage` false)))))

(event `Footstep`)

(event `self.ReceiveBeginPlay`
  (set `CharacterMovementComponent.MaxWalkSpeed` (`self.movementSpeed`) (`self.CharacterMovement`))
  (bind _asbp_first_person_character (cast `/Game/FirstPerson/Blueprints/BP_FirstPersonCharacter` (`GameplayStatics.GetPlayerCharacter` 0)))
  (set `self.As BP First Person Character` _asbp_first_person_character))

(event `self.ReceiveRadialDamage`
  (params (DamageReceived :type "Float (single-precision)") (DamageType :type "DamageType Object Reference") (Origin :type "Vector Structure") (HitInfo :type "HitResult Structure (by ref)") (InstigatedBy :type "Controller Object Reference") (DamageCauser :type "Actor Object Reference"))
  (`self.has been hit` DamageReceived))

(event `has been hit`
  (params (damage :type "Float (double-precision)"))
  (bind _output_get (set `self.health` (- (`self.health`) damage)))
  (if (<= _output_get 0.0)
    (set `self.dead` true)
    (`|ExecutionSequence`
      (:`then_0`
        ;[1 1 1] Points
        (if (not (`self.points consumed`))
          (set `self.points consumed` true)
          (bind _asbp_first_person_character (cast `/Game/FirstPerson/Blueprints/BP_FirstPersonCharacter` (`GameplayStatics.GetPlayerCharacter` 0)))
          (`/Game/FirstPerson/Blueprints/BP_FirstPersonCharacter.Multiply` _asbp_first_person_character)
          (`|ExecutionSequence`
            (:`then_0`
              (if (`/Game/GrappleHook/GrappleComponent.IsInUse?` (`/Game/FirstPerson/Blueprints/BP_FirstPersonCharacter.GrappleComponent` _asbp_first_person_character))
                (bind _multiplier (`/Game/FirstPerson/Blueprints/BP_FirstPersonCharacter.Multiplier` _asbp_first_person_character))
                (`self.AddPoints` _asbp_first_person_character (+ _multiplier 0.5))
                (set `self.GrappleMessage` true)
                (`KismetSystemLibrary.Delay` 1.0)
                (set `/Game/FirstPerson/Blueprints/BP_FirstPersonCharacter.Multiplier` (- _multiplier 0.5) _asbp_first_person_character)
                (elif (`NavMovementComponent.IsFalling` (`Character.CharacterMovement` _asbp_first_person_character))
                  (bind _multiplier_2 (`/Game/FirstPerson/Blueprints/BP_FirstPersonCharacter.Multiplier` _asbp_first_person_character))
                  (`self.AddPoints` _asbp_first_person_character (+ _multiplier_2 0.2))
                  (set `self.MidAirMessage` true)
                  (`KismetSystemLibrary.Delay` 1.0)
                  (set `/Game/FirstPerson/Blueprints/BP_FirstPersonCharacter.Multiplier` (- _multiplier_2 0.2) _asbp_first_person_character)
                  (else
                    (`self.AddPoints` _asbp_first_person_character _multiplier_2 :!label _label)))))
            (:`then_1`
              (if (and (== (`/Game/FirstPerson/Blueprints/BP_FirstPersonCharacter.Weapon` _asbp_first_person_character) 2) (not (`/Game/FirstPerson/Blueprints/BP_FirstPersonCharacter.bIsAiming` _asbp_first_person_character)))
                (`self.AddPoints` _asbp_first_person_character (+ _multiplier_2 0.3))
                (set `self.NoScopeMessage` true)
                (`KismetSystemLibrary.Delay` 1.0)
                (set `/Game/FirstPerson/Blueprints/BP_FirstPersonCharacter.Multiplier` (- _multiplier_2 0.3) _asbp_first_person_character)
                (else
                  (goto _label)))))))
      (:`then_1`
        (set `CharacterMovementComponent.MaxWalkSpeed` 0.0 (`self.CharacterMovement`))
        (`ActorComponent.Deactivate` (`self.AI_Behaviour`))
        (`ActorComponent.Deactivate` (`self.CharacterMovement`))
        (`KismetSystemLibrary.Delay` 1.1)
        (set `self.dead` false)
        (`self.K2_DestroyActor`)))
    (else
      (bind _returnvalue (`NiagaraFunctionLibrary.SpawnSystemAtLocation` "/Game/Vfx/Ns_sparks.Ns_sparks" (`self.K2_GetActorLocation` self)))
      (`PrimitiveComponent.SetRenderCustomDepth` _returnvalue true))))

(event `attack`
  (`|ExecutionSequence`
    (:`then_0`
      (set `self.isAttacking` true)
      (`KismetSystemLibrary.Delay` (`self.attack speed`))
      (bind _asbp_first_person_character (cast `/Game/FirstPerson/Blueprints/BP_FirstPersonCharacter` (`GameplayStatics.GetPlayerCharacter` 0)))
      (if (<= (`KismetMathLibrary.VSize` (- (`self.K2_GetActorLocation`) (`self.K2_GetActorLocation` _asbp_first_person_character))) (`self.melee range`))
        (`/Game/FirstPerson/Blueprints/BP_FirstPersonCharacter.Receive Damage` (`self.As BP First Person Character`) (`self.attack damage`))
        (`KismetSystemLibrary.Delay` (- 0.984 (`self.attack speed`)))
        (set `self.isAttacking` false)))
    (:`then_1`
      (if (`self.canPlaySound`)
        (set `self.canPlaySound` false)
        (`GameplayStatics.PlaySoundAtLocation` (`self.Sound`) (`self.K2_GetActorLocation`) (struct) 0.7 1.0 0.0 "/Game/AI/SettingsSound.SettingsSound" null null null)
        (`KismetSystemLibrary.Delay` 0.5)
        (set `self.canPlaySound` true)))))

(fn `recieve damage`
  (params (damage :type Integer)))

(fn `UserConstructionScript`)