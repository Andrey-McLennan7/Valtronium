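; Ranged enemy NPC that shoots projectiles at the first-person player.
; Attack sets a flag; Tick then halts movement, faces the player through a delay, and spawns a projectile from the left-hand socket before restoring speed.
; Projectile velocity is the unnormalized offset to above the player, scaled, so speed grows with distance.
; Tick also calls Footstep and briefly flashes flag-driven midair, grapple and no-scope messages on the player's HUD.
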(event `self.ReceiveBeginPlay`
  (set `CharacterMovementComponent.MaxWalkSpeed` (`self.movementSpeed_0`) (`self.CharacterMovement`))
  (set `self.health` 100.0)
  (set `self.MaxTimer` 0.4)
  (set `self.FootstepSound` "/Game/Audio/Enemy/MelleeRangedWalk_one_.MelleeRangedWalk_one_")
  (bind _asbp_first_person_character (cast `/Game/FirstPerson/Blueprints/BP_FirstPersonCharacter` (`GameplayStatics.GetPlayerCharacter` 0)))
  (set `self.As BP First Person Character_1` _asbp_first_person_character))

(event `self.attack`
  (set `self.attacking` true))

(event `self.ReceiveTick`
  (params (DeltaSeconds :type "Float (single-precision)"))
  (bind _returnvalue (`GameplayStatics.GetPlayerCharacter` 0))
  (bind _returnvalue_2 (`SceneComponent.GetSocketLocation` (`self.Mesh`) "Hand_LSocket"))
  (bind _returnvalue_3 (`self.K2_GetActorLocation` _returnvalue))
  (bind _returnvalue_4 (`KismetMathLibrary.FindLookAtRotation` (`self.K2_GetActorLocation`) _returnvalue_3))
  (bind _midairmessage (`/Game/UI/PointSystem/PointUI.Midairmessage` (`/Game/FirstPerson/Blueprints/BP_FirstPersonCharacter.PointHUD` (`self.As BP First Person Character_1`))))
  (bind _grapplemessage (`/Game/UI/PointSystem/PointUI.Grapplemessage` (`/Game/FirstPerson/Blueprints/BP_FirstPersonCharacter.PointHUD` (`self.As BP First Person Character_1`))))
  (bind _noscopemessage (`/Game/UI/PointSystem/PointUI.Noscopemessage` (`/Game/FirstPerson/Blueprints/BP_FirstPersonCharacter.PointHUD` (`self.As BP First Person Character_1`))))
  ;[1 1 1] Attacking sequence (rotate then attack)
  (`|ExecutionSequence`
    (:`then_0`
      (`self.Footstep`)
      (if (and (`self.attacking`) (`KismetSystemLibrary.IsValid` _returnvalue) (not (`self.dead`)))
        (set `CharacterMovementComponent.MaxWalkSpeed` 0.0 (`self.CharacterMovement`))
        (bind _output_get (set `self.look rot` _returnvalue_4))
        (`self.K2_SetActorRotation` (`KismetMathLibrary.MakeRotator` (.roll _output_get) 0.0 (.yaw _output_get)))
        (set `self.Return Value Y (Pitch)` (.pitch _output_get))
        (`KismetSystemLibrary.Delay` (`self.attack speed_0`))
        (bind _returnvalue_5 (`|SpawnActorFromClass` "/Game/AI/EnemyProjectiles/BP_Enemy_Projectile.BP_Enemy_Projectile_C" (`KismetMathLibrary.Conv_VectorToTransform` _returnvalue_2) "AlwaysSpawn" "MultiplyWithRoot" null null))
        (set `/Game/AI/EnemyProjectiles/BP_Enemy_Projectile.damage` (`KismetMathLibrary.Conv_IntToDouble` (`self.attack damage_0`)) _returnvalue_5)
        (set `MovementComponent.Velocity` (* (- (+ _returnvalue_3 (0.0 0.0 100.0)) _returnvalue_2) (60.0 60.0 60.0)) (`ProjectProjectile.ProjectileMovement` _returnvalue_5))
        (`self.K2_SetActorRotation` _returnvalue_5 _returnvalue_4 true)
        (set `self.attacking` false)
        (set `CharacterMovementComponent.MaxWalkSpeed` (`self.movementSpeed_0`) (`self.CharacterMovement`))
        (set `self.Sound` "/Game/Audio/Enemy/RanngedShot.RanngedShot")))
    (:`then_1`
      (if (`self.MidAirMessage`)
        (`Widget.SetRenderOpacity` _midairmessage 1.0)
        (`KismetSystemLibrary.Delay` 1.0)
        (`Widget.SetRenderOpacity` _midairmessage 0.0)
        (set `self.MidAirMessage` false)
        (elif (`self.GrappleMessage`)
          (`Widget.SetRenderOpacity` _grapplemessage 1.0)
          (`KismetSystemLibrary.Delay` 1.0)
          (`Widget.SetRenderOpacity` _grapplemessage 0.0)
          (set `self.GrappleMessage` false))))
    (:`then_2`
      (if (`self.NoScopeMessage`)
        (`Widget.SetRenderOpacity` _noscopemessage 1.0)
        (`KismetSystemLibrary.Delay` 1.0)
        (`Widget.SetRenderOpacity` _noscopemessage 0.0)
        (set `self.NoScopeMessage` false)))))

(fn `UserConstructionScript`)