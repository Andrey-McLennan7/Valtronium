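; BP_NPC_Exploder is a suicide-bomber NPC built on a parent NPC Blueprint, configured at BeginPlay with no patrolling, its own health, sounds and timer.
; A BPCExplosion component, initialized with a RadialForce and the NPC's Damage, performs the blast.
; Attack waits AttackSpeed before exploding, while Tick explodes once when Dead is set.
; Both paths spawn a Niagara explosion and destroy the actor; only the attack's effect enables custom depth rendering.
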(event `self.ReceiveBeginPlay`
  (`parent.ReceiveBeginPlay`)
  (set `self.shouldPatrol` false)
  (set `self.MaxTimer` 0.4)
  (set `self.FootstepSound` "/Game/Audio/Enemy/ExplosionWalk_one_.ExplosionWalk_one_")
  (`/Game/Weapons/BPC_Explosion.Init` (`self.BPC_Explosion`) (`self.RadialForce`))
  (set `/Game/Weapons/BPC_Explosion.BaseDamage` (`self.damage`) (`self.BPC_Explosion`))
  (set `self.Sound` "/Game/Audio/Enemy/ExploderBoom.ExploderBoom")
  (set `self.health` 50.0))

(event `self.ReceiveTick`
  (params (DeltaSeconds :type "Float (single-precision)"))
  (if (`self.dead`)
    (`/Engine/EditorBlueprintResources/StandardMacros.DoOnce` false
      (:`Completed`
        (`/Game/Weapons/BPC_Explosion.Explode` (`self.BPC_Explosion`))
        (`NiagaraFunctionLibrary.SpawnSystemAtLocation` "/Game/Vfx/Ns_explosion.Ns_explosion" (`self.K2_GetActorLocation` self))
        (`self.K2_DestroyActor`)))))

(event `self.attack`
  (set `self.isAttacking` true)
  (`KismetSystemLibrary.Delay` (`self.attack speed`))
  (`/Game/Weapons/BPC_Explosion.Explode` (`self.BPC_Explosion`))
  (`KismetSystemLibrary.PrintString` "explode")
  (bind _returnvalue (`NiagaraFunctionLibrary.SpawnSystemAtLocation` "/Game/Vfx/Ns_explosion.Ns_explosion" (`self.K2_GetActorLocation` self)))
  (`PrimitiveComponent.SetRenderCustomDepth` _returnvalue true)
  (`self.K2_DestroyActor`))

(fn `UserConstructionScript`
  (`parent.UserConstructionScript`))