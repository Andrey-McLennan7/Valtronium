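; BP_Rocket is a rocket weapon actor that explodes on impact or after a short time in flight.
; It hands its RadialForce to BPCExplosion at BeginPlay and delegates the blast to that component.
; A hit triggers the blast, spawns the Ns_explosion effect and destroys the actor.
; The Tick timeout only calls Explode, repeating every frame once elapsed, with no effect spawn or destroy in this graph.
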(event `self.ReceiveBeginPlay`
  (`/Game/Weapons/BPC_Explosion.Init` (`self.BPC_Explosion`) (`self.RadialForce`)))

(event `self.ReceiveHit`
  (params (MyComp :type "PrimitiveComponent Object Reference") (Other :type "Actor Object Reference") (OtherComp :type "PrimitiveComponent Object Reference") (bSelfMoved :type Boolean) (HitLocation :type "Vector Structure") (HitNormal :type "Vector Structure") (NormalImpulse :type "Vector Structure") (Hit :type "HitResult Structure (by ref)"))
  (`/Game/Weapons/BPC_Explosion.Explode` (`self.BPC_Explosion`))
  (`NiagaraFunctionLibrary.SpawnSystemAtLocation` "/Game/Vfx/Ns_explosion.Ns_explosion" HitLocation)
  (`self.K2_DestroyActor`))

(event `self.ReceiveTick`
  (params (DeltaSeconds :type "Float (single-precision)"))
  (bind _output_get (set `self.Timer` (+ (`self.Timer`) DeltaSeconds)))
  (if (>= _output_get 1.5)
    (`/Game/Weapons/BPC_Explosion.Explode` (`self.BPC_Explosion`))))

(fn `UserConstructionScript`)