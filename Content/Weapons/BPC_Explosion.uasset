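; Actor component that makes its owner explode, with sound, particle emitter, radial impulse and radial damage.
; Init supplies the radial force component that Explode fires and whose radius sets the damage area.
; Explode also stops the player's rocket launcher sound; rocket owners exclude the player from one damage pass and apply fixed damage to a nearby player.
; A final radial damage pass runs for every owner, on top of the branch-specific one.
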(event `self.ReceiveBeginPlay`
  (set `self.Owner` (`self.GetOwner`)))

(fn `Explode`
  (bind _returnvalue (`GameplayStatics.GetPlayerPawn` 0))
  (bind _owner (`self.Owner`))
  (bind _returnvalue_2 (`Actor.K2_GetActorLocation` (`self.Owner`)))
  (bind (_returnvalue_location _returnvalue_rotation) (`KismetMathLibrary.BreakTransform` (`Actor.GetTransform` _owner)))
  (bind _returnvalue_3 (`KismetMathLibrary.Vector_Distance` _returnvalue_2 (`Actor.K2_GetActorLocation` _returnvalue)))
  (`GameplayStatics.PlaySoundAtLocation` "/Game/Audio/rocketLauncher/Rocket_Sploded.Rocket_Sploded" (`Actor.K2_GetActorLocation` _owner) (struct) 0.5 1.0 0.0 null null null null)
  (bind _asbp_first_person_character (cast `/Game/FirstPerson/Blueprints/BP_FirstPersonCharacter` (`GameplayStatics.GetPlayerCharacter` 0)))
  (bind _rocketsound (`/Game/Weapons/BP_Rocket_Launcher_Component.RocketSOund` (`/Game/FirstPerson/Blueprints/BP_FirstPersonCharacter.RocketLauncherReference` _asbp_first_person_character)))
  (`/Engine/EditorBlueprintResources/StandardMacros.IsValid` _rocketsound
    (:`Is Valid`
      (`AudioComponent.Stop` _rocketsound))
    (:`Is Not Valid`
      _))
  (`GameplayStatics.SpawnEmitterAtLocation` null _returnvalue_location _returnvalue_rotation)
  (`|ExecutionSequence`
    (:`then_0`
      (`/Engine/EditorBlueprintResources/StandardMacros.IsValid` (`self.RadialComp`)
        (:`Is Valid`
          (`RadialForceComponent.FireImpulse` (`self.RadialComp`)))))
    (:`then_1`
      (cast `/Game/Weapons/BP_Rocket` (`self.Owner`)
        (:`then`
          (`GameplayStatics.ApplyRadialDamage` (`self.BaseDamage`) _returnvalue_2 (`RadialForceComponent.Radius` (`self.RadialComp`)) null (`|MakeArray` _returnvalue :!type "Actor Object Reference") null null)
          (`KismetSystemLibrary.PrintString` (`KismetStringLibrary.Conv_DoubleToString` _returnvalue_3))
          (if (< _returnvalue_3 400.0)
            (bind _asbp_first_person_character_2 (cast `/Game/FirstPerson/Blueprints/BP_FirstPersonCharacter` _returnvalue))
            (`/Game/FirstPerson/Blueprints/BP_FirstPersonCharacter.Receive Damage` _asbp_first_person_character_2 20.0)))
        (:`CastFailed`
          (`GameplayStatics.ApplyRadialDamage` :`BaseDamage` (`self.BaseDamage`) :`Origin` (`Actor.K2_GetActorLocation` (`self.Owner`)) :`DamageRadius` (`RadialForceComponent.Radius` (`self.RadialComp`)) :`DamageCauser` (`self.Owner`) :`InstigatedByController` null))))
    (:`then_2`
      (`GameplayStatics.ApplyRadialDamage` :`BaseDamage` (`self.BaseDamage`) :`Origin` (`Actor.K2_GetActorLocation` (`self.Owner`)) :`DamageRadius` (`RadialForceComponent.Radius` (`self.RadialComp`)) :`DamageCauser` (`self.Owner`) :`InstigatedByController` null))))

(fn `Init`
  (params (RadialComp :type "RadialForceComponent Object Reference"))
  (set `self.RadialComp` RadialComp))