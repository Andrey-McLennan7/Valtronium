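; Melee sword weapon component that sets its socket and fire rate on BeginPlay and detects hits during a swing.
; TriggerSword clears the hit list and loops a fast timer running box traces between Start and End sockets until StopTriggerSword.
; Tagged enemies join the ignore list and are passed to the FirstPersonCharacter with damage, with one hit sound per swing.
; Other physics-simulating hits receive an impulse along camera forward.
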(event `self.ReceiveBeginPlay`
  (`self.SetSocketName` "SwordSocket")
  (`parent.ReceiveBeginPlay`)
  (`self.SetFirerate` 0.3)
  (`self.K2_SetWorldLocation` (`self.K2_GetComponentLocation`)))

(event `TriggerSword`
  (`KismetArrayLibrary.Array_Clear` (`self.hit enemies`))
  (bind _returnvalue (`KismetSystemLibrary.K2_SetTimerDelegate` (delegate `SwordLinetrace`) 0.005 true))
  (set `self.TriggerSwordEvent` _returnvalue))

(event `SwordLinetrace`
  (bind _first_personcharacter (`self.First PersonCharacter`))
  (bind _outhit (`KismetSystemLibrary.BoxTraceSingle` (`self.GetSocketLocation` "Start") (`self.GetSocketLocation` "End") (`KismetMathLibrary.Conv_DoubleToVector` (`self.AreaOfEffect`)) (struct) "TraceTypeQuery1" false (`self.hit enemies`) "None" true (struct :`R` 1.0 :`A` 1.0) (struct :`G` 1.0 :`A` 1.0) 0.5))
  (bind (_bblockinghit _binitialoverlap _time _distance _location _impactpoint _normal _impactnormal _physmat _hitactor _hitcomponent) (`GameplayStatics.BreakHitResult` _outhit))
  ;[1 1 1] Hit tsting for enemy
  (`/Engine/EditorBlueprintResources/StandardMacros.IsValid` _hitactor
    (:`Is Valid`
      (if (`Actor.ActorHasTag` _hitactor "enemy")
        (`KismetArrayLibrary.Array_Append` (`self.hit enemies`) (`|MakeArray` _hitactor))
        (`/Engine/EditorBlueprintResources/StandardMacros.IsValid` _first_personcharacter
          (:`Is Valid`
            (`/Game/FirstPerson/Blueprints/BP_FirstPersonCharacter.hit enemy` _first_personcharacter _hitactor (`self.damage dealt`))
            (`/Engine/EditorBlueprintResources/StandardMacros.DoOnce` false :!label _label
              (:`Completed`
                (`GameplayStatics.PlaySound2D` "/Game/Audio/Sword/SwordHit.SwordHit" 0.6 1.0 0.0 null null)))))
        (else
          ;[0.05 0.05 0.05] Add impulse to objects with physics
          (if _bblockinghit
            (if (`self.IsSimulatingPhysics` _hitcomponent "None")
              (`self.AddImpulseAtLocation` _hitcomponent (* (`self.GetForwardVector` (`PlayerCameraManager.TransformComponent` (`GameplayStatics.GetPlayerCameraManager` 0))) (`self.Impact`)) _impactpoint "None"))))))))

(event `StopTriggerSword`
  (`KismetSystemLibrary.K2_ClearAndInvalidateTimerHandle` (`self.TriggerSwordEvent`))
  (goto _label :!via `Reset`))