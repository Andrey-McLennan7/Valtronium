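; Checkpoint actor that saves the player's respawn location when the first-person character overlaps its box.
; On BeginPlay it uses the current level name as the save slot, giving each level its own save.
; On overlap it loads or creates a BP_SaveGame, sets PlayerLocation to the checkpoint's own location, writes the slot and prints a notice.
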(event `self.ReceiveBeginPlay`
  (bind _returnvalue (`GameplayStatics.GetCurrentLevelName` true))
  (set `self.SaveGame` _returnvalue))

(event `self.Box.OnComponentBeginOverlap`
  (params (OverlappedComponent :type "PrimitiveComponent Object Reference") (OtherActor :type "Actor Object Reference") (OtherComp :type "PrimitiveComponent Object Reference") (OtherBodyIndex :type Integer) (bFromSweep :type Boolean) (SweepResult :type "HitResult Structure (by ref)"))
  (bind _returnvalue (`self.K2_GetActorLocation`))
  (cast `/Game/FirstPerson/Blueprints/BP_FirstPersonCharacter` OtherActor)
  (`KismetSystemLibrary.PrintString` "New Checkpoint")
  (bind _returnvalue_2 (`GameplayStatics.DoesSaveGameExist` (`self.SaveGame`)))
  (if _returnvalue_2
    (bind _returnvalue_3 (`GameplayStatics.LoadGameFromSlot` (`self.SaveGame`)))
    (bind _asbp_save_game (cast `/Game/SaveGame/BP_SaveGame` _returnvalue_3))
    (set `/Game/SaveGame/BP_SaveGame.PlayerLocation` _returnvalue _asbp_save_game)
    (`GameplayStatics.SaveGameToSlot` _asbp_save_game (`self.SaveGame`))
    (else
      (bind _returnvalue_4 (`GameplayStatics.CreateSaveGameObject` "/Game/SaveGame/BP_SaveGame.BP_SaveGame_C"))
      (set `/Game/SaveGame/BP_SaveGame.PlayerLocation` _returnvalue _returnvalue_4)
      (`GameplayStatics.SaveGameToSlot` _returnvalue_4 (`self.SaveGame`)))))

(fn `UserConstructionScript`)